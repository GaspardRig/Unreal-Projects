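; BP_trap2 is a trap actor that deals damage over time to BP_kaya while it overlaps the trap's Box.
; Entering the Box starts a looping one-second timer that calls DoDamages with Dmg and counts ticks in Compteur.
; The timer is cleared and the counter reset once Compteur reaches Duree or when any end overlap fires on the Box.
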(event `self.Box.OnComponentEndOverlap`
  (params (OverlappedComponent :type "PrimitiveComponent Object Reference") (OtherActor :type "Actor Object Reference") (OtherComp :type "PrimitiveComponent Object Reference") (OtherBodyIndex :type Integer))
  (`KismetSystemLibrary.K2_ClearAndInvalidateTimerHandle` (stale `self.Box.OnComponentBeginOverlap` _returnvalue) :!label _label)
  (set `self.compteur` 0))

(event `self.Box.OnComponentBeginOverlap`
  (params (OverlappedComponent :type "PrimitiveComponent Object Reference") (OtherActor :type "Actor Object Reference") (OtherComp :type "PrimitiveComponent Object Reference") (OtherBodyIndex :type Integer) (bFromSweep :type Boolean) (SweepResult :type "HitResult Structure (by ref)"))
  (bind _asbp_kaya (cast `/Game/Character/BP_kaya` OtherActor))
  (bind _returnvalue (`KismetSystemLibrary.K2_SetTimerDelegate` (delegate `dodmg`) 1.0 true)))

(event `dodmg`
  (if (< (`self.compteur`) (`self.duree`))
    (`/Game/Character/BP_kaya.do_damages` (stale `self.Box.OnComponentBeginOverlap` _asbp_kaya) (`self.dmg`))
    (`/Engine/EditorBlueprintResources/StandardMacros.IncrementInt` (`self.compteur`))
    (else
      (goto _label))))

(fn `UserConstructionScript`)
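; BP_door is an interactable swinging door that the player opens and closes with the use input.
; A trigger box enables input on the door while a BP_kaya actor overlaps it and disables it on exit.
; A timeline plays or reverses based on IsClosed, adding its yaw to the DoorC rotation cached at BeginPlay.
; Each timeline update also recomputes IsClosed from the current timeline value.
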(event `self.ReceiveBeginPlay`
  (set `self.rotation` (`SceneComponent.RelativeRotation` (`self.door_c`))))

(event `self.Box.OnComponentBeginOverlap`
  (params (OverlappedComponent :type "PrimitiveComponent Object Reference") (OtherActor :type "Actor Object Reference") (OtherComp :type "PrimitiveComponent Object Reference") (OtherBodyIndex :type Integer) (bFromSweep :type Boolean) (SweepResult :type "HitResult Structure (by ref)"))
  (cast `/Game/Character/BP_kaya` OtherActor)
  (`self.EnableInput` (`GameplayStatics.GetPlayerController` 0)))

(event `self.Box.OnComponentEndOverlap`
  (params (OverlappedComponent :type "PrimitiveComponent Object Reference") (OtherActor :type "Actor Object Reference") (OtherComp :type "PrimitiveComponent Object Reference") (OtherBodyIndex :type Integer))
  (cast `/Game/Character/BP_kaya` OtherActor)
  (`self.DisableInput` (`GameplayStatics.GetPlayerController` 0)))

(event `InputAction|use`
  (params (Key :type "Key Structure"))
  (bind (_rotation_roll _rotation_pitch _rotation_yaw) (`KismetMathLibrary.BreakRotator` (`self.rotation`)))
  (:`Pressed`
    (if (`self.is_closed`)
      (bind (_direction _rotation_timeline) (`Timeline|Timeline_0` :!label _label)
        (:`Update`
          (`SceneComponent.K2_SetRelativeRotation` (`self.door_c`) (`KismetMathLibrary.MakeRotator` _rotation_roll _rotation_pitch (+ _rotation_timeline _rotation_yaw)) false false)
          (set `self.is_closed` (< _rotation_timeline 1.0))))
      (else
        (goto _label :!via `Reverse`)))))

(fn `UserConstructionScript`)